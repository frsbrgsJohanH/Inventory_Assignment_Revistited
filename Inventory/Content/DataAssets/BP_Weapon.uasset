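; BP_Weapon is a data-driven weapon actor that can be placed in the world and interacted with.
; Its construction script checks for a valid DataAsset, then SetVariables copies name, damage and static mesh from the PDA_ItemBase asset, so the weapon updates when placed or moved.
; Interact only destroys the actor and returns false, and the event graph holds no active logic.
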(event EventBeginPlay)

(event Collision|EventActorBeginOverlap
  (params (OtherActor :type Actor%20Object%20Reference)))

(event EventTick
  (params (DeltaSeconds :type Float%20%28single-precision%29)))

(fn ConstructionScript
  ;[0.3694 0.07496 1] When Placed/Moved in world. This script is called.
  (if (Utilities|IsValid (Variables|Default|GetDataAsset))
    (CallFunction|SetVariables (Variables|Default|GetDataAsset))))

(fn SetVariables
  (params (DataAsset :type PDA%20Item%20Base%20Object%20Reference))
  ;[0.558 0.004539 1] Get and Set Variables from PDA_ItemBase to weapon.
  (Variables|Default|SetName (Variables|/MyInventory/PDA_ItemBase.PDA_ItemBase_C|GetName DataAsset))
  (Variables|Default|SetDamage (Variables|/MyInventory/PDA_ItemBase.PDA_ItemBase_C|GetDamage DataAsset))
  (Components|StaticMesh|SetStaticMesh (Variables|Default|GetWeaponMesh) (Variables|/MyInventory/PDA_ItemBase.PDA_ItemBase_C|GetMesh DataAsset))
  (return))

(fn Interact
  (Actor|DestroyActor)
  (return false))